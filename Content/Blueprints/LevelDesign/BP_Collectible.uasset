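; BP_Collectible is a pickup that adds a point when BP_Character overlaps it and triggers the win screen at a score of three or more.
; Shortly after BeginPlay it caches the first BP_Platformer actor as GameMode, which holds the shared Score.
; Below the threshold the pickup destroys itself; otherwise it pauses the game, shows WBP_WinScreen1 and switches to UI-only input with a visible cursor.
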(event `self.ReceiveBeginPlay`
  (`KismetSystemLibrary.Delay` 0.2)
  (bind _outactors (`GameplayStatics.GetAllActorsOfClass` "/Game/Blueprints/Player/BP_Platformer.BP_Platformer_C"))
  (bind _output_get (set `self.GameMode` (`|GetArrayItem` _outactors)))
  (`/Engine/EditorBlueprintResources/StandardMacros.IsValid` _output_get
    (:`Is Valid`
      (`KismetSystemLibrary.PrintString` "success"))))

(event `self.ReceiveActorBeginOverlap`
  (params (OtherActor :type "Actor Object Reference"))
  (bind _returnvalue (`GameplayStatics.GetPlayerController` 0))
  (bind _gamemode (`self.GameMode`))
  (cast `/Game/Blueprints/Player/BP_Character` OtherActor)
  (bind _output_get (set `/Game/Blueprints/Player/BP_Platformer.Score` (+ (`/Game/Blueprints/Player/BP_Platformer.Score` _gamemode) 1) _gamemode))
  (if (>= _output_get 3)
    (`GameplayStatics.SetGamePaused` true)
    (bind _returnvalue_2 (`|CreateWidget` "/Game/Blueprints/Widgets/WBP_WinScreen1.WBP_WinScreen1_C"))
    (`UserWidget.AddToViewport` _returnvalue_2 0)
    (`WidgetBlueprintLibrary.SetInputMode_UIOnlyEx` _returnvalue null)
    (set `PlayerController.bShowMouseCursor` true _returnvalue)
    (else
      (`self.K2_DestroyActor`))))

(fn `UserConstructionScript`)