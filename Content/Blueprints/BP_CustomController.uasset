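; BP_CustomController is a pawn-style Blueprint that takes movement from two input sets, labeled left brain and right brain.
; Each set has its own forward and side axis events, which call AddMovementInput along the actor's forward and right vectors.
; Both sets drive the same actor identically, so their inputs combine.
; BeginPlay, Tick and the construction script are empty.
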(event `InputAxis|MoveForward2`
  (params (AxisValue :type "Float (single-precision)"))
  ;[1 1 1] Right brain movement
  (`Pawn.AddMovementInput` (`self.GetActorForwardVector`) AxisValue))

(event `InputAxis|MoveSide2`
  (params (AxisValue :type "Float (single-precision)"))
  ;[1 1 1] Right brain movement
  (`Pawn.AddMovementInput` (`self.GetActorRightVector`) AxisValue))

(event `InputAxis|MoveForward1`
  (params (AxisValue :type "Float (single-precision)"))
  ;[1 1 1] Left brain movement
  (`Pawn.AddMovementInput` (`self.GetActorForwardVector`) AxisValue))

(event `InputAxis|MoveSide1`
  (params (AxisValue :type "Float (single-precision)"))
  ;[1 1 1] Left brain movement
  (`Pawn.AddMovementInput` (`self.GetActorRightVector`) AxisValue))

(fn `UserConstructionScript`)