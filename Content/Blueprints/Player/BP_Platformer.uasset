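; BP_Platformer sets up each level for up to three players and provides level loading.
; After a short BeginPlay delay, it maps tagged PlayerStarts, then moves each BP_Character to the start matching its PlayerIndex.
; It then creates the GUI, resets score, unpauses, parses the level number from the map name and sets game-only input.
; LoadLevel opens a map by building its name from "Level" plus a number.
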(event `self.ReceiveBeginPlay`
  (bind _returnvalue (`GameplayStatics.GetPlayerController` 0))
  (`KismetSystemLibrary.Delay` 0.1)
  (bind _outactors (`GameplayStatics.GetAllActorsOfClass` "/Script/Engine.PlayerStart"))
  (for _array_element _outactors
    (switch `string` (`KismetStringLibrary.Conv_NameToString` (`|GetArrayItem` (`Actor.Tags` _array_element)))
      (:`PlayerStart1`
        (bind _output_get (set `self.PlayerStart1` _array_element)))
      (:`PlayerStart2`
        (bind _output_get_2 (set `self.PlayerStart2` _array_element)))
      (:`PlayerStart3`
        (bind _output_get_3 (set `self.PlayerStart3` _array_element)))))
  (bind _outactors_2 (`GameplayStatics.GetAllActorsOfClass` "/Game/Blueprints/Player/BP_Character.BP_Character_C"))
  (for _array_element_2 _outactors_2
    (switch `int` (`/Game/Blueprints/Player/BP_Character.PlayerIndex` _array_element_2)
      (:`0`
        (bind _output_get_4 (set `self.Player1` _array_element_2))
        (`self.K2_SetActorLocation` _output_get_4 (`self.K2_GetActorLocation` _output_get) false false))
      (:`1`
        (bind _output_get_5 (set `self.Player2` _array_element_2))
        (`self.K2_SetActorLocation` _output_get_5 (`self.K2_GetActorLocation` _output_get_2) false false))
      (:`2`
        (bind _output_get_6 (set `self.Player3` _array_element_2))
        (`self.K2_SetActorLocation` _output_get_6 (`self.K2_GetActorLocation` _output_get_3) false false))))
  (bind _returnvalue_2 (`|CreateWidget` "/Game/Blueprints/Widgets/WBP_GUI.WBP_GUI_C"))
  (`UserWidget.AddToViewport` _returnvalue_2 0)
  (set `self.Score` 0)
  (`GameplayStatics.SetGamePaused` false)
  (bind _returnvalue_3 (`GameplayStatics.GetCurrentLevelName` true))
  (bind _returnvalue_4 (`KismetStringLibrary.Mid` _returnvalue_3 5 2))
  (set `self.CurrentLevel` (`KismetStringLibrary.Conv_StringToInt` _returnvalue_4))
  (set `/Game/Blueprints/Widgets/WBP_GUI.Level Text` (`KismetStringLibrary.Concat_StrStr` "Level " _returnvalue_4) _returnvalue_2)
  (`WidgetBlueprintLibrary.SetInputMode_GameOnly` _returnvalue)
  (set `PlayerController.bShowMouseCursor` false _returnvalue))

(fn `LoadLevel`
  (params (Level :type Integer))
  (bind _returnvalue (`KismetStringLibrary.Concat_StrStr` "Level" (`KismetStringLibrary.Conv_IntToString` Level)))
  (`KismetSystemLibrary.PrintString` _returnvalue)
  (`GameplayStatics.OpenLevel` (`KismetStringLibrary.Conv_StringToName` _returnvalue)))

(fn `UserConstructionScript`)