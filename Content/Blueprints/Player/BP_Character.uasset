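; Player character Blueprint that drives two "brain" characters, left and right, from separate P1 and P2 movement axes.
; Only the instance with PlayerIndex 0 routes input, looking up the first actor tagged Brain1 or Brain2 on each axis event.
; It casts that actor to BP_Character and calls its MoveForwardBack or MoveLeftRight event, which adds movement input along the actor's forward or right vector.
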(event `self.ReceiveBeginPlay`)

(event `InputAxis|MoveForwardP1`
  (params (AxisValue :type "Float (single-precision)"))
  ;[1 1 1] Left brain move
  (if (== (`self.PlayerIndex`) 0)
    (bind _outactors (`GameplayStatics.GetAllActorsWithTag` "Brain1"))
    (bind _asbp_character (cast `/Game/Blueprints/Player/BP_Character` (`|GetArrayItem` _outactors)))
    (`self.MoveForwardBack` _asbp_character AxisValue)))

(event `InputAxis|MoveSideP1`
  (params (AxisValue :type "Float (single-precision)"))
  ;[1 1 1] Left brain move
  (if (== (`self.PlayerIndex`) 0)
    (bind _outactors (`GameplayStatics.GetAllActorsWithTag` "Brain1"))
    (bind _asbp_character (cast `/Game/Blueprints/Player/BP_Character` (`|GetArrayItem` _outactors)))
    (`self.MoveLeftRight` _asbp_character AxisValue)))

(event `InputAxis|MoveForwardP2`
  (params (AxisValue :type "Float (single-precision)"))
  ;[1 1 1] Right brain movement
  (if (== (`self.PlayerIndex`) 0)
    (bind _outactors (`GameplayStatics.GetAllActorsWithTag` "Brain2"))
    (bind _asbp_character (cast `/Game/Blueprints/Player/BP_Character` (`|GetArrayItem` _outactors)))
    (`self.MoveForwardBack` _asbp_character AxisValue)))

(event `InputAxis|MoveSideP2`
  (params (AxisValue :type "Float (single-precision)"))
  ;[1 1 1] Right brain movement
  (if (== (`self.PlayerIndex`) 0)
    (bind _outactors (`GameplayStatics.GetAllActorsWithTag` "Brain2"))
    (bind _asbp_character (cast `/Game/Blueprints/Player/BP_Character` (`|GetArrayItem` _outactors)))
    (`self.MoveLeftRight` _asbp_character AxisValue)))

(event `MoveForwardBack`
  (params (InputScale :type "Float (single-precision)"))
  (`self.AddMovementInput` (`self.GetActorForwardVector`) InputScale))

(event `MoveLeftRight`
  (params (InputScale :type "Float (single-precision)"))
  (`self.AddMovementInput` (`self.GetActorRightVector`) InputScale))

(fn `UserConstructionScript`)