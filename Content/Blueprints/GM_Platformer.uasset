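; GM_Platformer is the platformer game mode that spawns and possesses the player pawns at startup.
; On BeginPlay it spawns the main character at its spawn point for player controller 0.
; It then spawns the Left Brain pawn and creates a second local player to possess it.
; A matching Right Brain spawn for a third local player exists but is disconnected, so it never runs.
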(event `self.ReceiveBeginPlay`
  (bind _returnvalue (`|SpawnActorFromClass` "/Game/Blueprints/BP_Character.BP_Character_C" (`self.Spawnpoint`) "Undefined" "MultiplyWithRoot" null null))
  (`Controller.Possess` (`GameplayStatics.GetPlayerController` 0) _returnvalue)
  ;[1 1 1] Spawn Left Brain
  (bind _returnvalue_2 (`|SpawnActorFromClass` "/Game/Blueprints/BP_Leftbrain.BP_Leftbrain_C" (`self.LeftSpawnPoint`) "AlwaysSpawn" "MultiplyWithRoot" null null))
  (bind _returnvalue_3 (`GameplayStatics.CreatePlayer` -1))
  (`Controller.Possess` _returnvalue_3 _returnvalue_2))

(fn `UserConstructionScript`)