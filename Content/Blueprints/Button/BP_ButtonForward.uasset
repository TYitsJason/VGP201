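; BP_ButtonForward is an overlap button that drives the player-index-0 BP_Character forward while it is held down.
; Shortly after BeginPlay it searches all BP_Character actors and caches the one with that index as ControlledCharacter.
; Any BP_Character beginning or ending overlap toggles Pressed, and Tick calls MoveForwardBack on the cached character while Pressed is true.
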(event `self.ReceiveBeginPlay`
  (`KismetSystemLibrary.Delay` 0.2)
  (bind _outactors (`GameplayStatics.GetAllActorsOfClass` "/Game/Blueprints/Player/BP_Character.BP_Character_C"))
  (for _array_element _outactors
    (if (== (`/Game/Blueprints/Player/BP_Character.PlayerIndex` _array_element) 0)
      (set `self.ControlledCharacter` _array_element)
      (break))))

(event `self.ReceiveActorBeginOverlap`
  (params (OtherActor :type "Actor Object Reference"))
  (cast `/Game/Blueprints/Player/BP_Character` OtherActor)
  (set `self.Pressed` true))

(event `self.ReceiveActorEndOverlap`
  (params (OtherActor :type "Actor Object Reference"))
  (cast `/Game/Blueprints/Player/BP_Character` OtherActor)
  (set `self.Pressed` false))

(event `self.ReceiveTick`
  (params (DeltaSeconds :type "Float (single-precision)"))
  (if (`self.Pressed`)
    (`/Game/Blueprints/Player/BP_Character.MoveForwardBack` (`self.ControlledCharacter`) 1.0)))

(fn `UserConstructionScript`)